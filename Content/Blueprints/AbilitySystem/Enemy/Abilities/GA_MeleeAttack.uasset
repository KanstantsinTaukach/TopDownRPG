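; Enemy melee attack Gameplay Ability that turns the avatar toward its combat target and plays a random tagged attack montage.
; A gameplay event matching the montage tag triggers a small radius check at the montage's combat socket for live, non-friendly players.
; Hits receive damage and a MeleeImpact gameplay cue.
; The ability ends on a hit or montage finish or interruption, without stopping the montage.
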(event Ability|EventActivateAbility
  (bind _returnvalue (Ability|GetAvatarActorfromActorInfo))
  (bind _returnvalue_2 (Ability|GetAvatarActorfromActorInfo))
  (bind _returnvalue_3 (Ability|GetAvatarActorfromActorInfo))
  (bind _returnvalue_4 (Class|TDRPGEnemyInterface|GetCombatTarget(Message) _returnvalue_2))
  (bind _astdrpgcombat_interface (Utilities|Casting|CastToTDRPGCombatInterface _returnvalue_2))
  (Class|TDRPGCombatInterface|UpdateFacingTarget _astdrpgcombat_interface (Transformation|GetActorLocation _returnvalue_4))
  (bind _returnvalue_5 (Class|TDRPGCombatInterface|GetAttackMontages(Message) (Ability|GetAvatarActorfromActorInfo)))
  (Variables|Default|SetTaggedMontage (Class|TDRPGDamageGameplayAbility|GetRandomTaggedMontagefromAttay _returnvalue_5))
  (|PlayMontageandWaitProxy "None" (.Montage (Utilities|Struct|BreakTaggedMontage (Variables|Default|GetTaggedMontage))) 1.0 "None" false 1.0 0.0 false
    (:then
      (Ability|Tasks|WaitGameplayEvent (.MontageTag (Utilities|Struct|BreakTaggedMontage (Variables|Default|GetTaggedMontage))) 0
        (:EventReceived
          (bind _returnvalue_6 (Class|TDRPGCombatInterface|GetCombatSocketLocation(Message) _returnvalue (.SocketTag (Utilities|Struct|BreakTaggedMontage (Variables|Default|GetTaggedMontage)))))
          (bind _outoverlappingactors (Class|TDRPGAbilitySystemLibrary|GetLivePlayersWithinRadius _returnvalue (Utilities|Array|MakeArray _returnvalue) 45.0 _returnvalue_6))
          (for _array_element _outoverlappingactors
            (if (Class|TDRPGAbilitySystemLibrary|IsNotFriend _returnvalue_3 _array_element)
              (Class|TDRPGDamageGameplayAbility|CauseDamage _array_element)
              (Class|GameplayAbility|ExecuteGameplayCuewithParams "(TagName=\"GameplayCue.MeleeImpact\")" (Ability|GameplayCue|MakeGameplayCueParameters :AggregatedSourceTags (GameplayTags|MakeGameplayTagContainerfromTag (.MontageTag (Utilities|Struct|BreakTaggedMontage (Variables|Default|GetTaggedMontage)))) :Location _returnvalue_6 :EffectCauser _returnvalue_3 :SourceObject _returnvalue_4))
              (Ability|EndAbility))))))
    (:OnCompleted
      (Ability|EndAbility :!label _label))
    (:OnInterrupted
      (goto _label))
    (:OnCancelled
      (goto _label))))