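; GA_RangedAttack is an enemy gameplay ability that fires a projectile at the avatar's combat target.
; On activation it caches the target's location, turns the avatar to face it and plays a random tagged attack montage.
; A gameplay event matching the montage's tag triggers SpawnProjectile from its socket tag, with optional pitch override, then ends the ability.
; Montage completion, interruption or cancellation also ends it.
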(event Ability|EventActivateAbility
  (bind _returnvalue (Ability|GetAvatarActorfromActorInfo))
  (bind _returnvalue_2 (Class|TDRPGEnemyInterface|GetCombatTarget(Message) _returnvalue))
  (bind _output_get (Variables|Default|SetTargetLocation (Transformation|GetActorLocation _returnvalue_2)))
  (Class|TDRPGCombatInterface|UpdateFacingTarget(Message) _returnvalue _output_get)
  (bind _returnvalue_3 (Class|TDRPGCombatInterface|GetAttackMontages(Message) (Ability|GetAvatarActorfromActorInfo)))
  (Variables|Default|SetTaggedMontage (Class|TDRPGDamageGameplayAbility|GetRandomTaggedMontagefromAttay _returnvalue_3))
  (|PlayMontageandWaitProxy "None" (.Montage (Utilities|Struct|BreakTaggedMontage (Variables|Default|GetTaggedMontage))) 1.0 "None" false 1.0 0.0 false
    (:then
      (Ability|Tasks|WaitGameplayEvent (.MontageTag (Utilities|Struct|BreakTaggedMontage (Variables|Default|GetTaggedMontage))) 0 true
        (:EventReceived
          (Class|TDRPGProjectileSpell|SpawnProjectile (Variables|Default|GetTargetLocation) (.SocketTag (Utilities|Struct|BreakTaggedMontage (Variables|Default|GetTaggedMontage))) (Variables|Default|GetbShouldOverridePitch) (Variables|Default|GetPitchOverride))
          (Ability|EndAbility))))
    (:OnCompleted
      (Ability|EndAbility :!label _label))
    (:OnInterrupted
      (goto _label))
    (:OnCancelled
      (goto _label))))