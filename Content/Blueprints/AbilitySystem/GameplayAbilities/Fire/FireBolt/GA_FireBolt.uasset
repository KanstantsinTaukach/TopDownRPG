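; GA_FireBolt is the gameplay ability that casts a fire bolt projectile toward the point under the mouse.
; On activation, a target data task supplies the hit location, which is stored and used to turn the avatar through the combat interface.
; It then plays the cast montage and waits for that montage's gameplay event to spawn the projectile at the stored target, ending after a short delay.
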(event Ability|EventActivateAbility
  (bind _datahandle (|TargetDataUnderMouse)
    (:ValidData
      (bind _output_get (Variables|Default|SetProjectileTargetLocation (.Location (Collision|BreakHitResult (Ability|TargetData|GetHitResultfromTargetData _datahandle)))))
      (bind _astdrpgcombat_interface (Utilities|Casting|CastToTDRPGCombatInterface (Ability|GetAvatarActorfromActorInfo))
        (:then
          (Class|TDRPGCombatInterface|UpdateFacingTarget _astdrpgcombat_interface _output_get))
        (:CastFailed
          _))
      (|PlayMontageandWaitProxy "None" "/Game/Assets/Characters/Aura/Animations/Abilities/AM_Aura_Cast_FireBolt.AM_Aura_Cast_FireBolt" 1.0 "None" true 1.0 0.0 false
        (:then
          (Ability|Tasks|WaitGameplayEvent "(TagName=\"Event.Montage.FireBolt\")" 0
            (:EventReceived
              (Class|TDRPGProjectileSpell|SpawnProjectile (Variables|Default|GetProjectileTargetLocation))
              (Utilities|FlowControl|Delay 0.2)
              (Ability|EndAbility))))))))